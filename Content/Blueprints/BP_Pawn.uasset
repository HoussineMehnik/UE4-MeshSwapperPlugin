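; BP_Pawn is a test-style pawn Blueprint that exercises a MeshSwapperComponent, which plays keyframed static mesh animations.
; Its only live logic prints each animation notify tag to the screen briefly.
; The finished-playing event and construction script are empty.
; Unconnected nodes lay out the component and animation API for playback control and keyframe queries, but never execute.
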(event OnFinishedPlaying(MeshSwapperComponent))

(event OnAnimationNotifyEvent(MeshSwapperComponent)
  (params (NotifyTag :type String) (FrameIndex :type Integer))
  (Development|PrintString NotifyTag true true "(R=0.000000,G=0.660000,B=1.000000,A=1.000000)" 0.5))

(fn ConstructionScript)